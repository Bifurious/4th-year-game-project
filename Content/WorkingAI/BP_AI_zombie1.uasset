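; Zombie AI character that wanders, chases a seen FPSCharacter and dies from damage.
; BeginPlay sets a slow walk speed and seeds Blackboard range, behavior and start location through the BBData helper.
; PawnSensing drives AIMoveTo chasing and a sight flag cleared by retriggerable delay; while clear, Tick issues delayed random reachable moves around its current location.
; Depleted health triggers Died once, stops audio, ragdolls the mesh, then destroys the actor.
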(event `self.ReceiveBeginPlay`
  (bind (_returnvalue _returnvalue2) (`self.BB_Data` "StartLocation"))
  (bind (_returnvalue_2 _returnvalue2_2) (`self.BB_Data` "WanderingRange"))
  (bind (_returnvalue_3 _returnvalue2_3) (`self.BB_Data` "DefaultBehavior"))
  (set `self.Start_Location` (`self.K2_GetActorLocation`))
  (`BlackboardComponent.SetValueAsFloat` _returnvalue_2 _returnvalue2_2 (`self.Max_WanderDistance`))
  (`BlackboardComponent.SetValueAsEnum` _returnvalue_3 _returnvalue2_3 (`self.Default_Behavior`))
  (`BlackboardComponent.SetValueAsVector` _returnvalue _returnvalue2 (`self.Start_Location`))
  (set `CharacterMovementComponent.MaxWalkSpeed` 100.0 (`self.CharacterMovement`)))

(event `self.ReceiveAnyDamage`
  (params (Damage :type "Float (single-precision)") (DamageType :type "DamageType Object Reference") (InstigatedBy :type "Controller Object Reference") (DamageCauser :type "Actor Object Reference"))
  (bind _mesh (`self.Mesh`))
  (set `self.Health` (- (`self.Health`) Damage))
  (if (< (`self.Health`) 1.0)
    (`/Engine/EditorBlueprintResources/StandardMacros.DoOnce` false
      (:`Completed`
        (`self.died`)
        (`ActorComponent.Deactivate` (`self.Audio`))
        (`PrimitiveComponent.SetCollisionEnabled` _mesh "PhysicsOnly")
        (`PrimitiveComponent.SetSimulatePhysics` _mesh true)
        (`PrimitiveComponent.SetCollisionEnabled` (`self.CapsuleComponent`) "NoCollision")
        (`ActorComponent.Deactivate` (`self.Audio`))
        (`KismetSystemLibrary.Delay` 5.0)
        (`self.K2_DestroyActor`)))))

(event `self.PawnSensing.OnSeePawn`
  (params (Pawn :type "Pawn Object Reference"))
  (bind _asfpscharacter (cast `FPSCharacter` Pawn))
  (`|ExecutionSequence`
    (:`then_0`
      (set `self.seeenemy` true)
      (`|AIMoveTo` self (0.0 0.0 0.0) _asfpscharacter))
    (:`then_1`
      (`KismetSystemLibrary.RetriggerableDelay` 0.5)
      (set `self.seeenemy` false))))

(event `self.ReceiveTick`
  (params (DeltaSeconds :type "Float (single-precision)"))
  (if (not (`self.seeenemy`))
    (`KismetSystemLibrary.Delay` (`KismetMathLibrary.RandomFloatInRange` 2.0 5.0))
    (`|AIMoveTo` self (`NavigationSystemV1.K2_GetRandomReachablePointInRadius` (`self.K2_GetActorLocation`) 1000.0 null null) null)))

(fn `BB_Data`
  (params (KeyName :type Name))
  (returns (ReturnValue :type "BlackboardComponent Object Reference") (ReturnValue2 :type Name))
  (return (`AIBlueprintHelperLibrary.GetBlackboard` (`AIBlueprintHelperLibrary.GetAIController` self)) (`KismetSystemLibrary.MakeLiteralName` KeyName)))

(fn `UserConstructionScript`)