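; Destructible actor that steps through HP-based damage states, swapping mesh, particle and sound, with overflow damage skipping states.
; The construction script clamps state data and derives HP from the starting state onward.
; On death it hides or shows its last state, plays effects and spawns randomized debris as runtime-built mesh actors with self-destroy timers.
; A looping timer polls those handles before conditionally destroying the owner, checking active particles and audio.
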(event `self.ReceiveAnyDamage`
  (params (Damage :type "Float (single-precision)") (DamageType :type "DamageType Object Reference") (InstigatedBy :type "Controller Object Reference") (DamageCauser :type "Actor Object Reference"))
  (bind _returnvalue (`KismetMathLibrary.FTrunc` Damage))
  (if (> (`self.CurrentHP`) 0)
    (bind _output_get (set `self.CurrentHP` (- (`self.CurrentHP`) _returnvalue)))
    (if (<= _output_get 0)
      (`self.BeginDeath`)
      (else
        (bind (_nextstate _nextstatehp) (`self.CalculateNextState` _returnvalue))
        (set `self.CurrentState` _nextstate)
        (set `self.CurrentStateHP` _nextstatehp)
        (`self.GoToState` (`self.CurrentState`))))))

(fn `BeginDeath`
  (bind _returnvalue (`KismetArrayLibrary.Array_LastIndex` (`self.States`)))
  (if (`self.bMakeLastStatePermanent`)
    ;[1 1 1] Just make sure actor is in the last state.
    (if (!= (`self.CurrentState`) _returnvalue)
      (`self.GoToState` _returnvalue))
    (else
      ;[1 1 1] We need to fake our death until debris actors are not destroyed.
      (`SceneComponent.SetHiddenInGame` (`self.StaticMesh`) true true)
      (`self.SetActorEnableCollision` false)))
  (`self.SetParticleIfValid` (`self.DeathParticle`))
  (`self.SetSoundIfValid` (`self.DeathSound`))
  (if (> (`KismetArrayLibrary.Array_Length` (`self.DebrisActorPropertiesArray`)) 0)
    (`KismetSystemLibrary.K2_SetTimer` self "DebrisActorsTimer" (`self.DebrisActorsCheckInterval`) true)
    (for _array_element (`self.DebrisActorPropertiesArray`)
      (`self.SpawnDebrisActor` _array_element))
    (else
      (`self.ConditionalDestroyActor` true true))))

(fn `CalculateNextState`
  (params (Damage :type Integer))
  (returns (NextState :type Integer) (NextStateHP :type Integer))
  (locals (DamageLeft :type Integer) (StateHP :type Integer) (LocalState :type Integer) (LoopValue :type Integer))
  (set `local.DamageLeft` Damage)
  (set `local.LocalState` (`self.CurrentState`))
  (set `local.StateHP` (`self.CurrentStateHP`))
  ;[1 1 1] We loop just to bo sure we ommited enough states if taken damage is bigger than current state's hp.
  (while (and (> (`local.DamageLeft`) 0) (< (`local.LocalState`) (`KismetArrayLibrary.Array_Length` (`self.States`))))
    (bind _output_get (set `local.LoopValue` (- (`local.DamageLeft`) (`local.StateHP`))))
    (if (< _output_get 0)
      (set `local.StateHP` (- (`local.StateHP`) (`local.DamageLeft`)))
      (set `local.DamageLeft` -1)
      (else
        (set `local.DamageLeft` (`local.LoopValue`))
        (bind _result (`/Engine/EditorBlueprintResources/StandardMacros.IncrementInt` (`local.LocalState`))
          (:`  `
            (bind _statehp (`self.GetStateHP` _result))
            (set `local.StateHP` _statehp))))))
  (return (`local.LocalState`) (`local.StateHP`)))

(fn `CalculateStartingHP`
  (params (StartingStateHP :type Integer))
  (returns (CalculatedHP :type Integer))
  (if (or (== (`self.StartingHP`) 0) (!= (`self.StartingState`) (`self.CurrentState`)) (== (`self.StartingHP`) (`self.LastCSStartingHP`)))
    (return StartingStateHP)
    (else
      (return (`KismetMathLibrary.Clamp` (`self.StartingHP`) 0 StartingStateHP)))))

(fn `ClampStateValues`
  (params (State :type "/Game/DestructionSystem/Blueprints/Structs/DestructionSystemActorState Structure") (ArrayIndex :type Integer))
  (returns (ClampedState :type "/Game/DestructionSystem/Blueprints/Structs/DestructionSystemActorState Structure"))
  (locals (StateName :type Text))
  (bind (_name _staticmesh _transitionparticle _transitionsound _hp) (break `/Game/DestructionSystem/Blueprints/Structs/DestructionSystemActorState` State))
  ;[1 1 1] If state name is empty, we create a simple name based on array index.
  (bind _output_get (set `local.StateName` _name))
  (if (`KismetTextLibrary.TextIsEmpty` _output_get)
    (set `local.StateName` (`KismetTextLibrary.Conv_StringToText` (`KismetStringLibrary.BuildString_Int` "" "State" ArrayIndex))))
  (bind _structout (setmembers `/Game/DestructionSystem/Blueprints/Structs/DestructionSystemActorState` :`StructRef` State :`Name` (`local.StateName`) :`HP` (`KismetMathLibrary.Max` _hp)))
  (return _structout))

(fn `ConditionalDestroyActor`
  (params (bCheckParticleSystem :type Boolean) (bCheckAudio :type Boolean))
  (`|ExecutionSequence`
    (:`then_0`
      ;[1 1 1] We check this so particles or sound are not destroyed until finished.
      (if bCheckParticleSystem
        (if (`ActorComponent.IsActive` (`self.ParticleSystem`))
          (return))))
    (:`then_1`
      (if bCheckAudio
        (if (`ActorComponent.IsActive` (`self.Audio`))
          (return))))
    (:`then_2`
      (`self.K2_DestroyActor`)
      (return))))

(fn `DebrisActorsTimer`
  (locals (ActorsToRemove :type "Array of Actor Object Reference") (HandlesToRemove :type "Array of TimerHandle Structure"))
  (for _array_element (`self.DebrisActorsTimersHandles`)
    (if (not (`KismetSystemLibrary.K2_IsTimerActiveHandle` _array_element))
      (`KismetArrayLibrary.Array_Add` (`local.HandlesToRemove`) _array_element)))
  (for _array_element_2 (`local.HandlesToRemove`)
    (`KismetArrayLibrary.Array_RemoveItem` (`self.DebrisActorsTimersHandles`) _array_element_2))
  (if (== (`KismetArrayLibrary.Array_Length` (`self.DebrisActorsTimersHandles`)) 0)
    (`KismetSystemLibrary.K2_ClearTimer` self "DebrisActorsTimer")
    (`self.ConditionalDestroyActor` true true)))

(fn `GetStateHP`
  (params (StateIndex :type Integer))
  (returns (StateHP :type Integer))
  (if (and (>= StateIndex 0) (< StateIndex (`KismetArrayLibrary.Array_Length` (`self.States`))))
    (return (`.HP_15_3864D4F44D72A6B72DB6D2AA241E94E6` (break `/Game/DestructionSystem/Blueprints/Structs/DestructionSystemActorState` (`|GetArrayItem` (`self.States`) StateIndex))))
    (else
      (return -1))))

(fn `GoToState`
  (params (StateIndex :type Integer))
  (bind (_name _staticmesh _transitionparticle _transitionsound) (break `/Game/DestructionSystem/Blueprints/Structs/DestructionSystemActorState` (`|GetArrayItem` (`self.States`) StateIndex)))
  (if (< StateIndex (`KismetArrayLibrary.Array_Length` (`self.States`)))
    (`self.SetMeshIfValid` _staticmesh)
    (`self.SetParticleIfValid` _transitionparticle)
    (`self.SetSoundIfValid` _transitionsound)))

(fn `SetDebrisActorCollision`
  (params (Actor :type "Actor Object Reference") (StaticMeshComponent :type "StaticMeshComponent Object Reference") (bCollisionEnabled :type Boolean))
  (`self.SetActorEnableCollision` Actor bCollisionEnabled)
  (if bCollisionEnabled
    (`PrimitiveComponent.SetCollisionObjectType` StaticMeshComponent "ECC_PhysicsBody")
    (`PrimitiveComponent.SetCollisionResponseToChannel` StaticMeshComponent "ECC_Pawn" "ECR_Ignore")
    (`PrimitiveComponent.SetCollisionResponseToChannel` StaticMeshComponent "ECC_Vehicle" "ECR_Ignore")))

(fn `SetDebrisActorProperties`
  (params (Actor :type "Actor Object Reference") (StaticMeshComponent :type "StaticMeshComponent Object Reference") (StaticMesh :type "StaticMesh Object Reference") (Location :type "Vector Structure") (Rotation :type "Rotator Structure") (Scale :type "Vector Structure") (Impulse :type "Vector Structure") (DeathTimer :type "Float (double-precision)") (bPhysicsEnabled :type Boolean) (bCollisionEnabled :type Boolean) (bCastShadows :type Boolean))
  (`/Engine/EditorBlueprintResources/StandardMacros.IsValid` Actor
    (:`Is Valid`
      (`self.SetDebrisActorCollision` Actor StaticMeshComponent bCollisionEnabled)
      (`self.K2_AddActorWorldOffset` Actor Location false false)
      (`self.K2_AddActorWorldRotation` Actor Rotation false false)
      (`self.SetActorScale3D` Actor Scale)
      (bind _returnvalue (`KismetSystemLibrary.K2_SetTimer` Actor "K2_DestroyActor" DeathTimer))
      (`KismetArrayLibrary.Array_Add` (`self.DebrisActorsTimersHandles`) _returnvalue)
      (`/Engine/EditorBlueprintResources/StandardMacros.IsValid` StaticMeshComponent
        (:`Is Valid`
          (bind _returnvalue_2 (`StaticMeshComponent.SetStaticMesh` StaticMeshComponent StaticMesh))
          (if _returnvalue_2
            (`PrimitiveComponent.SetSimulatePhysics` StaticMeshComponent bPhysicsEnabled)
            (`PrimitiveComponent.SetCastShadow` StaticMeshComponent bCastShadows)
            (if bPhysicsEnabled
              (`PrimitiveComponent.AddImpulseAtLocation` StaticMeshComponent Impulse (`self.K2_GetActorLocation` Actor) "None"))))))))

(fn `SetMeshIfValid`
  (params (StaticMeshAsset :type "StaticMesh Object Reference"))
  (`/Engine/EditorBlueprintResources/StandardMacros.IsValid` (`self.StaticMesh`)
    (:`Is Valid`
      (`/Engine/EditorBlueprintResources/StandardMacros.IsValid` StaticMeshAsset
        (:`Is Valid`
          (`StaticMeshComponent.SetStaticMesh` (`self.StaticMesh`) StaticMeshAsset)
          (return))
        (:`Is Not Valid`
          (return))))
    (:`Is Not Valid`
      (return))))

(fn `SetParticleIfValid`
  (params (ParticleSystemAsset :type "ParticleSystem Object Reference"))
  (`/Engine/EditorBlueprintResources/StandardMacros.IsValid` (`self.ParticleSystem`)
    (:`Is Valid`
      (`/Engine/EditorBlueprintResources/StandardMacros.IsValid` ParticleSystemAsset
        (:`Is Valid`
          (`ParticleSystemComponent.SetTemplate` (`self.ParticleSystem`) ParticleSystemAsset)
          (`ActorComponent.Activate` (`self.ParticleSystem`) true)
          (return))
        (:`Is Not Valid`
          (return))))
    (:`Is Not Valid`
      (return))))

(fn `SetSoundIfValid`
  (params (SoundAsset :type "SoundBase Object Reference"))
  (`/Engine/EditorBlueprintResources/StandardMacros.IsValid` (`self.Audio`)
    (:`Is Valid`
      (`/Engine/EditorBlueprintResources/StandardMacros.IsValid` SoundAsset
        (:`Is Valid`
          (`AudioComponent.SetSound` (`self.Audio`) SoundAsset)
          (`ActorComponent.Activate` (`self.Audio`) true)
          (return))
        (:`Is Not Valid`
          (return))))
    (:`Is Not Valid`
      (return))))

(fn `SpawnDebrisActor`
  (params (Properties :type "/Game/DestructionSystem/Blueprints/Structs/DestructionSystemDebrisActorProperties Structure"))
  (bind (_debrismesh _spawnoffset _spawnimpulse _destroydelay _bphysicsenabled _bcollisionenabled _bcastshadows) (break `/Game/DestructionSystem/Blueprints/Structs/DestructionSystemDebrisActorProperties` Properties))
  (bind _returnvalue (`|SpawnActorFromClass` "/Script/Engine.Actor" (`KismetMathLibrary.MakeTransform` (0.0 0.0 0.0)) "AlwaysSpawn" "OverrideRootScale" self null))
  (`/Engine/EditorBlueprintResources/StandardMacros.IsValid` _returnvalue
    (:`Is Valid`
      (bind _returnvalue_2 (`AddComponent|NODE_AddStaticMeshComponent-1` :`self` _returnvalue))
      (`self.SetDebrisActorProperties` _returnvalue _returnvalue_2 _debrismesh (+ (`self.RandomVectorInRange` _spawnoffset) (.location (`self.GetTransform`))) (.rotation (`self.GetTransform`)) (.scale (`self.GetTransform`)) (`self.RandomVectorInRange` _spawnimpulse) (`self.RandomFloatInRange` _destroydelay) _bphysicsenabled _bcollisionenabled _bcastshadows))))

(fn `UserConstructionScript`
  (bind _states (`self.States`))
  (bind _startingstate (`self.StartingState`))
  ;[1 1 1] We need to check if there are any states and clamp starting state if it's out of array bounds.
  (if (== (`KismetArrayLibrary.Array_Length` _states) 0)
    (set `self.StartingState` -1)
    (else
      (set `self.StartingState` (`KismetMathLibrary.Clamp` (`self.StartingState`) 0 (`KismetArrayLibrary.Array_LastIndex` _states)))
      (for (_array_element _array_index) (`self.States`)
        ;[1 1 1] First, we need to make sure state values are not out of bounds.
        (bind _clampedstate (`self.ClampStateValues` _array_element _array_index))
        (`KismetArrayLibrary.Array_Set` (`self.States`) _array_index _clampedstate)
        (if (>= _array_index (`self.StartingState`))
          (set `self.CurrentHP` (+ (`self.CurrentHP`) (`.HP_15_3864D4F44D72A6B72DB6D2AA241E94E6` (break `/Game/DestructionSystem/Blueprints/Structs/DestructionSystemActorState` _array_element))))))
      (bind _statehp (`self.GetStateHP` (`self.StartingState`)))
      (bind _calculatedhp (`self.CalculateStartingHP` _statehp))
      (bind _output_get (set `self.StartingHP` _calculatedhp))
      (bind _output_get_2 (set `self.CurrentStateHP` _output_get))
      (set `self.LastCSStartingHP` _output_get_2)
      (set `self.CurrentState` _startingstate)
      (`self.GoToState` _startingstate))))